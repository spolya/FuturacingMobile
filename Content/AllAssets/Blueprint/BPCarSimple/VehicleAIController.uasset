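; AI controller that drives an AllCarPawn vehicle along a SplineTrack.
; On BeginPlay it takes its instigator as the car and seeks a random non-LiderSpline track.
; GetRightAxis steers toward a look-ahead spline point, while GetForwardAxis cuts throttle as a farther point strays from straight ahead, except at low speed.
; Tick line traces override this, steering away from side obstacles and, after a delay, inverting throttle when blocked ahead.
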(event EventBeginPlay
  (bind _asall_car_pawn (Utilities|Casting|CastToAllCarPawn (Game|GetInstigator)))
  (Variables|Default|SetParentVehicle _asall_car_pawn)
  (bind _outactors (Actor|GetAllActorsOfClass "/Game/AllAssets/Blueprint/BPCarSimple/SplineTrack.SplineTrack_C" :!label _label))
  (if (Utilities|Array|IsValidIndex _outactors)
    (Utilities|IsValid (Utilities|Array|Get(acopy) _outactors (Math|Random|RandomIntegerinRange 0 (Utilities|Array|LastIndex _outactors)))
      (:Is%20Valid
        (if (Variables|/Game/AllAssets/Blueprint/BPCarSimple/SplineTrack.SplineTrack_C|GetLiderSpline (Utilities|Array|Get(acopy) _outactors (Math|Random|RandomIntegerinRange 0 (Utilities|Array|LastIndex _outactors))))
          (goto _label)
          (else
            (Variables|Default|SetGetSplineActor (Utilities|Array|Get(acopy) _outactors (Math|Random|RandomIntegerinRange 0 (Utilities|Array|LastIndex _outactors))))))))))

(event EventTick
  (params (DeltaSeconds :type Float%20%28single-precision%29))
  (bind _parentvehicle (Variables|Default|GetParentVehicle))
  (bind _parentvehicle_2 (Variables|Default|GetParentVehicle))
  (bind _parentvehicle_3 (Variables|Default|GetParentVehicle))
  (bind _parentvehicle_4 (Variables|Default|GetParentVehicle))
  (bind _body (Variables|/Game/AllAssets/Blueprint/BPCarSimple/AllCarPawn.AllCarPawn_C|GetBody _parentvehicle))
  (bind _body_2 (Variables|/Game/AllAssets/Blueprint/BPCarSimple/AllCarPawn.AllCarPawn_C|GetBody _parentvehicle_3))
  (bind _body_3 (Variables|/Game/AllAssets/Blueprint/BPCarSimple/AllCarPawn.AllCarPawn_C|GetBody _parentvehicle_4))
  (bind _returnvalue (Transformation|GetWorldLocation _body_2))
  (bind _returnvalue_2 (Transformation|GetWorldLocation _body_3))
  (bind _returnvalue_3 (Transformation|GetWorldLocation _body))
  (bind _returnvalue_4 (+ _returnvalue_3 "0, 0,50.000000"))
  (bind _returnvalue_5 (+ _returnvalue "0, 0,50.000000"))
  (bind _returnvalue_6 (+ _returnvalue_2 "0, 0,50.000000"))
  (Utilities|FlowControl|Sequence
    (:then_0
      (bind _returnvalue_7 (Collision|LineTraceForObjects _returnvalue_5 (+ (* (Math|Vector|GetForwardVector _body_2) 5e+02) _returnvalue_5) (Utilities|Array|MakeArray "ObjectTypeQuery1") false (Utilities|Array|MakeArray _parentvehicle_3) "None"))
      (if _returnvalue_7
        (Utilities|FlowControl|Delay 2.0)
        (Variables|Default|SetForwardHit true)
        (Default|SetForwardVar _parentvehicle_2 (* (CallFunction|GetForwardAxis) -1.0))
        (Default|SetRightVar _parentvehicle_2 (* (CallFunction|GetRightAxis 9e+01) 1.0))
        (Variables|Default|SetRightHit false)
        (Variables|Default|SetLeftHit false)
        (else
          (Utilities|FlowControl|Delay 0.2)
          (Variables|Default|SetForwardHit false))))
    (:then_1
      (if (not (Variables|Default|GetForwardHit))
        (bind _returnvalue_8 (Collision|LineTraceForObjects _returnvalue_6 (+ (* (Math|Vector|GetForwardVector _body_3) 5e+02) _returnvalue_6 (* (Math|Vector|GetRightVector _body_3) 5e+02)) (Utilities|Array|MakeArray "ObjectTypeQuery1" "ObjectTypeQuery5") false (Utilities|Array|MakeArray _parentvehicle_4) "None"))
        (bind _output_get (Variables|Default|SetRightHit _returnvalue_8))
        (if _output_get
          (Default|SetRightVar (Variables|Default|GetParentVehicle) -1.0))))
    (:then_2
      (if (not (Variables|Default|GetForwardHit))
        (bind _returnvalue_9 (Collision|LineTraceForObjects _returnvalue_4 (+ (* (Math|Vector|GetForwardVector _body) 5e+02) _returnvalue_4 (* (Math|Vector|GetRightVector _body) -5e+02)) (Utilities|Array|MakeArray "ObjectTypeQuery1" "ObjectTypeQuery5") false (Utilities|Array|MakeArray _parentvehicle) "None"))
        (bind _output_get_2 (Variables|Default|SetLeftHit _returnvalue_9))
        (if _output_get_2
          (Default|SetRightVar (Variables|Default|GetParentVehicle) 1.0))))
    (:then_3
      (if (not (Variables|Default|GetForwardHit))
        (Default|SetForwardVar (Variables|Default|GetParentVehicle) (CallFunction|GetForwardAxis))
        (if (and (Math|Boolean|Equal(Boolean) (Variables|Default|GetRightHit) false) (Math|Boolean|Equal(Boolean) (Variables|Default|GetLeftHit) false))
          (Default|SetRightVar (Variables|Default|GetParentVehicle) (CallFunction|GetRightAxis 9e+01))
          (Development|PrintString "Hello" true true "(R=0.000000,G=0.660000,B=1.000000,A=1.000000)" 0.0))))))

(fn ConstructionScript)

(fn GetRightAxis
  (params (MaxAngle :type Float%20%28single-precision%29))
  (bind _parentvehicle (Variables|Default|GetParentVehicle))
  (bind _body (Variables|/Game/AllAssets/Blueprint/BPCarSimple/AllCarPawn.AllCarPawn_C|GetBody _parentvehicle))
  (Utilities|IsValid (Variables|Default|GetGetSplineActor)
    (:Is%20Valid
      (return (Math|Float|MapRangeUnclamped (.Yaw (Math|Rotator|BreakRotator (Math|Rotator|Delta(Rotator) (Math|Rotator|FindLookatRotation (Transformation|GetWorldLocation _body) (Default|PointForwardonSpline (Variables|Default|GetGetSplineActor) 2500 (Variables|Default|GetParentVehicle))) (Transformation|GetWorldRotation _body)))) MaxAngle (* MaxAngle -1.0) 1.0 -1.0)))))

(fn GetForwardAxis
  (bind _parentvehicle (Variables|Default|GetParentVehicle))
  (bind _parentvehicle_2 (Variables|Default|GetParentVehicle))
  (bind _getsplineactor (Variables|Default|GetGetSplineActor))
  (bind _returnvalue (Default|PointForwardonSpline _getsplineactor 5500 _parentvehicle))
  (bind _body (Variables|/Game/AllAssets/Blueprint/BPCarSimple/AllCarPawn.AllCarPawn_C|GetBody _parentvehicle_2))
  (bind (_x _y) (Math|Vector|BreakVector _returnvalue))
  (bind _returnvalue_2 (Math|Vector|GetForwardVector _body))
  (bind _returnvalue_3 (Transformation|GetWorldLocation _body))
  (bind _returnvalue_4 (* _returnvalue_2 5500))
  (bind _returnvalue_5 (+ _returnvalue_4 _returnvalue_3))
  (bind (_x_2 _y_2) (Math|Vector|BreakVector _returnvalue_5))
  (Utilities|IsValid (Variables|Default|GetGetSplineActor)
    (:Is%20Valid
      (return (Math|Float|SelectFloat 1.0 (Math|Float|MapRangeClamped (Math|Vector|VectorLength (- (Math|Vector|MakeVector _x _y 0.0) (Math|Vector|MakeVector _x_2 _y_2 0.0))) 5e+02 (Variables|Default|GetMaxLengthToSpline) 1.0 (Variables|Default|GetMinThrottle)) (< (Math|Float|Absolute(Float) (Default|GetSpeed (Variables|Default|GetParentVehicle))) (Variables|Default|GetMinSpeed)))))))