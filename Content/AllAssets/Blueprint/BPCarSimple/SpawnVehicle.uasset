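; Spawn point actor that creates either the player's car or an AI enemy car at BeginPlay, chosen by the AIVehicle flag.
; It reads car and weapon catalogs and player selections from GameModeFuturacing.
; The player gets the selected car and gun, possession and a HUD; AI gets a random car, the first gun and a default controller.
; Tuning arrays set vehicle and weapon stats, with AI cars using the player-selected car's tuning.
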(event EventBeginPlay
  (CallFunction|LoadVeriables)
  (CallFunction|SpawnEnemyandGG))

(fn ConstructionScript)

(fn LoadVeriables
  (bind _asgame_mode_futuracing (Utilities|Casting|CastToGameModeFuturacing (Game|GetGameMode)))
  (Variables|Default|SetCar (Variables|/Game/AllAssets/Blueprint/GameModeFuturacing.GameModeFuturacing_C|GetMagazineCar _asgame_mode_futuracing))
  (Variables|Default|SetGun (Variables|/Game/AllAssets/Blueprint/GameModeFuturacing.GameModeFuturacing_C|GetMagazineWeapon _asgame_mode_futuracing))
  (Variables|Default|SetNumberCar (Variables|/Game/AllAssets/Blueprint/GameModeFuturacing.GameModeFuturacing_C|GetPlayerCarIndex _asgame_mode_futuracing))
  (Variables|Default|SetNumberGun (Variables|/Game/AllAssets/Blueprint/GameModeFuturacing.GameModeFuturacing_C|GetPlayerWeaponIndex _asgame_mode_futuracing)))

(fn UpdateParametr
  (params (InputPin :type All%20Car%20Pawn%20Object%20Reference))
  (for (_array_element _array_index) (.TuningPercentARR (Utilities|Struct|BreakParametrArrStruct (Variables|Default|GetLokalParam)))
    (switch int _array_index
      (:0
        (Variables|/Game/AllAssets/Blueprint/BPCarSimple/AllCarPawn.AllCarPawn_C|SetAcceleration InputPin _array_element))
      (:1
        (Variables|/Game/AllAssets/Blueprint/BPCarSimple/AllCarPawn.AllCarPawn_C|SetMaxSpeed InputPin _array_element))
      (:2
        (Variables|/Game/AllAssets/Blueprint/BPCarSimple/AllCarPawn.AllCarPawn_C|SetSteering InputPin _array_element))
      (:3
        (Variables|/Game/AllAssets/Blueprint/BPCarSimple/AllCarPawn.AllCarPawn_C|SetHealth InputPin _array_element)
        (Default|UpdateHealthWidget InputPin)))))

(fn UpdateParametrGun
  (params (self2 :type All%20Car%20Pawn%20Object%20Reference))
  (bind _gun (Variables|Default|GetGun))
  (bind _numbergun (Variables|Default|GetNumberGun))
  (bind _childactor (Variables|/Game/AllAssets/Blueprint/BPCarSimple/AllCarPawn.AllCarPawn_C|GetChildActor self2))
  (bind _gun_2 (Variables|Default|GetGun))
  (bind _output (Utilities|Array|Get(acopy) _gun _numbergun))
  (bind _output_2 (Utilities|Array|Get(acopy) _gun_2))
  (bind _childactor_2 (Variables|/Script/Engine.ChildActorComponent|GetChildActor _childactor))
  (bind (_gunbp _structureparametr) (Utilities|Struct|BreakGunStructArr _output))
  (bind (_gunbp_2 _structureparametr_2) (Utilities|Struct|BreakGunStructArr _output_2))
  (if (Variables|Default|GetAIVehicle)
    (ChildActorComponent|SetChildActorClass _childactor _gunbp_2)
    (bind _asweapon_bptest (Utilities|Casting|CastToweaponBPtest _childactor_2))
    (for (_array_element _array_index) (.TuningPercentARR (Utilities|Struct|BreakParametrArrStruct _structureparametr_2))
      (switch int _array_index
        (:0
          (Variables|/Game/AllAssets/Blueprint/WeaponsBP/weaponBPtest.weaponBPtest_C|SetTimeAttack _asweapon_bptest _array_element))
        (:1
          (Variables|/Game/AllAssets/Blueprint/WeaponsBP/weaponBPtest.weaponBPtest_C|SetDamage _asweapon_bptest _array_element))
        (:2
          (Variables|/Game/AllAssets/Blueprint/WeaponsBP/weaponBPtest.weaponBPtest_C|SetTimeRotate _asweapon_bptest _array_element))
        (:3
          (Variables|/Game/AllAssets/Blueprint/WeaponsBP/weaponBPtest.weaponBPtest_C|SetLengthAttack _asweapon_bptest _array_element))))
    (else
      (ChildActorComponent|SetChildActorClass _childactor _gunbp)
      (bind _asweapon_bptest_2 (Utilities|Casting|CastToweaponBPtest _childactor_2))
      (for (_array_element_2 _array_index_2) (.TuningPercentARR (Utilities|Struct|BreakParametrArrStruct _structureparametr))
        (switch int _array_index_2
          (:0
            (Variables|/Game/AllAssets/Blueprint/WeaponsBP/weaponBPtest.weaponBPtest_C|SetTimeAttack _asweapon_bptest_2 _array_element_2))
          (:1
            (Variables|/Game/AllAssets/Blueprint/WeaponsBP/weaponBPtest.weaponBPtest_C|SetDamage _asweapon_bptest_2 _array_element_2))
          (:2
            (Variables|/Game/AllAssets/Blueprint/WeaponsBP/weaponBPtest.weaponBPtest_C|SetTimeRotate _asweapon_bptest_2 _array_element_2))
          (:3
            (Variables|/Game/AllAssets/Blueprint/WeaponsBP/weaponBPtest.weaponBPtest_C|SetLengthAttack _asweapon_bptest_2 _array_element_2)))))))

(fn SpawnEnemyandGG
  (bind _returnvalue (Transformation|GetActorTransform))
  (bind _car (Variables|Default|GetCar))
  (bind _numbercar (Variables|Default|GetNumberCar))
  (bind _car_2 (Variables|Default|GetCar))
  (bind _output (Utilities|Array|Get(acopy) _car _numbercar))
  (bind (_vehiclemesh _structparametr) (Utilities|Struct|BreakVehicleStructArr _output))
  (if (Utilities|Array|IsValidIndex (Variables|Default|GetCar))
    (Variables|Default|SetLokalParam _structparametr)
    (if (Variables|Default|GetAIVehicle)
      (bind _asall_car_pawn (Utilities|Casting|CastToAllCarPawnClass (.VehicleMesh (Utilities|Struct|BreakVehicleStructArr (Utilities|Array|Get(acopy) _car_2 (Math|Random|RandomIntegerinRange 0 (Utilities|Array|LastIndex _car_2)))))))
      (bind _returnvalue_2 (Game|SpawnActorfromClass _asall_car_pawn _returnvalue "Undefined" 0 (Utilities|Array|Get(acopy) (.TuningPercentARR (Utilities|Struct|BreakParametrArrStruct (Variables|Default|GetLokalParam)))) (Utilities|Array|Get(acopy) (.TuningPercentARR (Utilities|Struct|BreakParametrArrStruct (Variables|Default|GetLokalParam))) 1) (Utilities|Array|Get(acopy) (.TuningPercentARR (Utilities|Struct|BreakParametrArrStruct (Variables|Default|GetLokalParam))) 2) (Utilities|Array|Get(acopy) (.TuningPercentARR (Utilities|Struct|BreakParametrArrStruct (Variables|Default|GetLokalParam))) 3) 0))
      (Pawn|SpawnDefaultController _returnvalue_2)
      (bind _output_get (Variables|Default|SetVehicleActor _returnvalue_2))
      (CallFunction|UpdateParametr _output_get)
      (CallFunction|UpdateParametrGun _output_get)
      (else
        (bind _asall_car_pawn_2 (Utilities|Casting|CastToAllCarPawnClass _vehiclemesh))
        (bind _returnvalue_3 (Game|SpawnActorfromClass _asall_car_pawn_2 _returnvalue "Undefined" 0 (Utilities|Array|Get(acopy) (.TuningPercentARR (Utilities|Struct|BreakParametrArrStruct (Variables|Default|GetLokalParam)))) (Utilities|Array|Get(acopy) (.TuningPercentARR (Utilities|Struct|BreakParametrArrStruct (Variables|Default|GetLokalParam))) 1) (Utilities|Array|Get(acopy) (.TuningPercentARR (Utilities|Struct|BreakParametrArrStruct (Variables|Default|GetLokalParam))) 2) (Utilities|Array|Get(acopy) (.TuningPercentARR (Utilities|Struct|BreakParametrArrStruct (Variables|Default|GetLokalParam))) 3) 0))
        (Pawn|Possess (Game|GetPlayerController 0) _returnvalue_3)
        (Variables|Default|SetVehicleActor _returnvalue_3)
        (CallFunction|UpdateParametr _returnvalue_3)
        (CallFunction|UpdateParametrGun _returnvalue_3)
        (bind _returnvalue_4 (UserInterface|CreateWidget "/Game/AllAssets/Blueprint/BPCarSimple/HUDplayer/PlayerHUDwidget.PlayerHUDwidget_C"))
        (UserInterface|Viewport|AddtoViewport _returnvalue_4 0)))))