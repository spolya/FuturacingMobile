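; Drivable car pawn with a physics-simulated body, flip-recovery roll torque and a toggleable control-rotation camera.
; Construction spawns a custom simple component and mesh per WheelSetup entry, with getters exposing suspension, input and speed.
; Tick uses speed and wheel state to drive body materials, wheel spin and height, and engine and skid audio.
; Damage updates a 3D health widget; death, braking or exceeding max speed zeroes throttle.
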(event EventTick
  (params (DeltaSeconds :type Float%20%28single-precision%29))
  (bind _returnvalue (CallFunction|GetSpeed))
  (bind _returnvalue_2 (CallFunction|GetSpeed))
  (bind _forwardaxisvolue (CallFunction|GetForwardInput))
  (bind _returnvalue_3 (CallFunction|GetSpeed))
  (bind _body (Variables|Default|GetBody))
  (bind _tireskidaudio (Variables|Default|GetTireSkidAudio))
  (bind _returnvalue_4 (Math|Float|Absolute(Float) _returnvalue))
  (bind _returnvalue_5 (Math|Float|Absolute(Float) _returnvalue_3))
  (if (Variables|SetupVehicle|GetUsePhysics)
    (Rendering|Material|SetScalarParameterValueonMaterials _body "ForwardVector" (Variables|Private|GetForwardAxisVolue))
    (Rendering|Material|SetScalarParameterValueonMaterials _body "Speed" (Math|Float|Clamp(Float) (CallFunction|GetSpeed) -1.0))
    (CallFunction|AddRotationWheel)
    (Development|PrintString (Utilities|String|ToString(Float) (CallFunction|GetSpeed)) true true "(R=0.000000,G=0.660000,B=1.000000,A=1.000000)" 0.0)
    (Audio|Parameter|SetFloatParameter (Variables|Default|GetEngineAudio) "Speed" _returnvalue_5 :!class /Script/Engine.AudioComponent)
    (Audio|Components|Audio|SetPitchMultiplier (Variables|Default|GetEngineAudio) (* (/ _returnvalue_5 (Variables|Parametr|GetMaxSpeed)) 2.0))
    (Components|Activation|SetActive _tireskidaudio (or (and (> (Math|Float|Absolute(Float) (CallFunction|GetRightInput)) 0.0) (> (Math|Float|Absolute(Float) (CallFunction|GetSpeed)) 1e+01)) (or (and (> _returnvalue_2 0.0) (< _forwardaxisvolue 0.0)) (and (< _returnvalue_2 0.0) (> _forwardaxisvolue 0.0)))) false)
    (Audio|Parameter|SetFloatParameter _tireskidaudio "Speed" _returnvalue_4 :!class /Script/Engine.AudioComponent)
    (Audio|Components|Audio|SetPitchMultiplier (Variables|Default|GetTireSkidAudio) (* (/ _returnvalue_4 (Variables|Parametr|GetMaxSpeed)) 2.0))
    (else
      (Utilities|FlowControl|DoOnce false
        (:Completed
          (for _array_element (Variables|Private|GetWheelsArr)
            (Transformation|SetRelativeLocation _array_element "0, 0, 0" true true)))))))

(event EventBeginPlay
  (bind _usephysics (Variables|SetupVehicle|GetUsePhysics))
  ;[1 1 1] Инициализация
  (Development|ExecuteConsoleCommand (Game|GetPlayerController 0) "Stat FPS" 0)
  (CallFunction|UpdateHealthWidget)
  (if _usephysics
    (CallFunction|UsePhysicsCar _usephysics)))

(event Game|Damage|EventAnyDamage
  (params (Damage :type Float%20%28single-precision%29) (DamageType :type Damage%20Type%20Object%20Reference) (InstigatedBy :type Controller%20Object%20Reference) (DamageCauser :type Actor%20Object%20Reference))
  ;[0.2083 0.2083 0.2083 1 36] Урон и смерть машины
  (CallFunction|ApplayDamage Damage))

(event Input|ActionEvents|InputActionHandbreack
  (params (Key :type Key%20Structure))
  ;[1 1 1] Управление
)

(event Input|AxisEvents|InputAxisMoveForward
  (params (AxisValue :type Float%20%28single-precision%29))
  ;[1 1 1] Управление
  (Variables|Private|SetForwardAxisVolue AxisValue))

(event Input|AxisEvents|InputAxisMoveRight
  (params (AxisValue :type Float%20%28single-precision%29))
  ;[1 1 1] Управление
  (Variables|Private|SetRightAxisVolue AxisValue))

(event Input|AxisEvents|InputAxisRemoveRotate
  (params (AxisValue :type Float%20%28single-precision%29))
  ;[1 1 1] Переворот машины
  (if (not (Variables|Private|GetDeadCar))
    (Class|PrimitiveComponent|AddTorqueinRadians (Variables|Default|GetBody) (* (Math|Vector|GetForwardVector (Variables|Default|GetBody)) (* AxisValue 5e+01)) "None" true)))

(event Input|AxisEvents|InputAxisLookRight
  (params (AxisValue :type Float%20%28single-precision%29))
  (Pawn|Input|AddControllerYawInput AxisValue))

(event Input|AxisEvents|InputAxisLookUp
  (params (AxisValue :type Float%20%28single-precision%29))
  (Pawn|Input|AddControllerPitchInput AxisValue))

(event Input|KeyboardEvents|C
  (params (Key :type Key%20Structure))
  (bind _springarm (Variables|Default|GetSpringArm))
  (:Pressed
    (Utilities|FlowControl|FlipFlop
      (:A
        (Variables|/Script/Engine.SpringArmComponent|SetbUsePawnControlRotation _springarm true))
      (:B
        (Variables|/Script/Engine.SpringArmComponent|SetbUsePawnControlRotation _springarm false)))))

(fn ConstructionScript
  (Components|StaticMesh|SetStaticMesh (Variables|Default|GetBody) (Variables|SetupVehicle|GetStatickMeshBody))
  (Class|PrimitiveComponent|SetMassOverrideinKg (Variables|Default|GetBody) "None" (Variables|SetupVehicle|GetMassVehicle) true)
  (CallFunction|CreateWheels))

(fn WheelsLocation
  (for (_array_element _array_index) (Variables|Private|GetWheelsArr)
    (Transformation|AddLocalRotation _array_element (Math|Rotator|MakeRotator 0.0 (Variables|/Game/AllAssets/Blueprint/BPCarSimple/SimpleComponent.SimpleComponent_C|GetAngularVelocity (Utilities|Array|Get(acopy) (Variables|Private|GetComponentArr) _array_index)) 0.0) true true)
    (Transformation|SetWorldLocation _array_element (Math|Vector|MakeVector (.x (Transformation|GetWorldLocation _array_element)) (.y (Transformation|GetWorldLocation _array_element)) (.z (Variables|/Game/AllAssets/Blueprint/BPCarSimple/SimpleComponent.SimpleComponent_C|GetWheelLocation (Utilities|Array|Get(acopy) (Variables|Private|GetComponentArr) _array_index)))) true true)
    (Transformation|SetRelativeLocation _array_element (Math|Vector|MakeVector 0.0 0.0 (.z (Variables|/Script/Engine.SceneComponent|GetRelativeLocation _array_element))) true true)))

(fn UsePhysicsCar
  (params (UsePhysics :type Boolean))
  (bind _output_get (Variables|SetupVehicle|SetUsePhysics UsePhysics))
  (Physics|SetSimulatePhysics (Variables|Default|GetBody) _output_get)
  (if (Variables|SetupVehicle|GetUsePhysics)
    (Input|SetInputModeGameOnly (Game|GetPlayerController 0))))

(fn UpdateHealthWidget
  (bind _asdata_player_widget (Utilities|Casting|CastToDataPlayerWidget (UserInterface|GetUserWidgetObject (Variables|Default|Get3DWidget))))
  (Variables|/Game/AllAssets/Blueprint/BPCarSimple/DataPlayerWidget.DataPlayerWidget_C|SetParentCar _asdata_player_widget self)
  (bind _output_get (Variables|/Game/AllAssets/Blueprint/BPCarSimple/DataPlayerWidget.DataPlayerWidget_C|SetHealth _asdata_player_widget (Variables|Parametr|GetHealth)))
  (Variables|/Game/AllAssets/Blueprint/BPCarSimple/DataPlayerWidget.DataPlayerWidget_C|SetHealthMax _asdata_player_widget _output_get))

(fn ApplayDamage
  (params (DamageValue :type Float%20%28single-precision%29))
  (if (not (Variables|Private|GetDeadCar))
    (Variables|Parametr|SetHealth (- (Variables|Parametr|GetHealth) DamageValue))
    (if (> (Variables|Parametr|GetHealth) 0.0)
      (bind _asdata_player_widget (Utilities|Casting|CastToDataPlayerWidget (UserInterface|GetUserWidgetObject (Variables|Default|Get3DWidget))))
      (Variables|/Game/AllAssets/Blueprint/BPCarSimple/DataPlayerWidget.DataPlayerWidget_C|SetHealth _asdata_player_widget (Variables|Parametr|GetHealth))
      (else
        (Variables|Private|SetDeadCar true)
        (bind _asdata_player_widget_2 (Utilities|Casting|CastToDataPlayerWidget (UserInterface|GetUserWidgetObject (Variables|Default|Get3DWidget))))
        (Widget|SetVisibility (Variables|/Game/AllAssets/Blueprint/BPCarSimple/DataPlayerWidget.DataPlayerWidget_C|GetProgressBar_69 _asdata_player_widget_2) "Hidden")
        (Variables|/Game/AllAssets/Blueprint/BPCarSimple/DataPlayerWidget.DataPlayerWidget_C|SetHealth _asdata_player_widget_2 (Variables|Parametr|GetHealth))))))

(fn CreateWheels
  (for _array_element (Variables|SetupVehicle|GetWheelSetup)
    (bind _returnvalue (AddComponent|AddSimpleComponent false))
    (Utilities|Array|Add (Variables|Private|GetComponentArr) _returnvalue)
    (bind _output_get (LocalVariables|SetSceneComponent _returnvalue))
    (Variables|/Game/AllAssets/Blueprint/BPCarSimple/SimpleComponent.SimpleComponent_C|SetRadiusWheel _output_get (.Radius (Utilities|Struct|BreakWheelStructVehicle _array_element)))
    (Variables|/Game/AllAssets/Blueprint/BPCarSimple/SimpleComponent.SimpleComponent_C|SetuseSteer _output_get (.UseSteering (Utilities|Struct|BreakWheelStructVehicle _array_element)))
    (Variables|/Game/AllAssets/Blueprint/BPCarSimple/SimpleComponent.SimpleComponent_C|SetUseForce _output_get (.UseForce (Utilities|Struct|BreakWheelStructVehicle _array_element)))
    (Transformation|AttachComponentToComponent _output_get (Variables|Default|GetBody) (.SocketName (Utilities|Struct|BreakWheelStructVehicle _array_element)) "KeepRelative" "KeepRelative" "KeepRelative" true)
    (bind _returnvalue_2 (AddComponent|AddStaticMeshComponent false (Math|Transform|MakeTransform "0, 0, 0" "0, 0, 0" (Math|Vector|MakeVector 1.0 (Math|Float|SelectFloat -1.0 1.0 (.Inverting (Utilities|Struct|BreakWheelStructVehicle _array_element))) 1.0))))
    (Components|StaticMesh|SetStaticMesh _returnvalue_2 (.WheelMesh (Utilities|Struct|BreakWheelStructVehicle _array_element)))
    (Utilities|Array|Add (Variables|Private|GetWheelsArr) _returnvalue_2)
    (Collision|SetCollisionEnabled _returnvalue_2 "NoCollision")
    (Transformation|AttachComponentToComponent _returnvalue_2 (LocalVariables|GetSceneComponent) "None" "KeepRelative" "KeepRelative" "KeepRelative" true)))

(fn GetLengthSuspension
  (return (Variables|SetupVehicle|GetLengthSuspension)))

(fn GetForceSuspension
  (return (Variables|SetupVehicle|GetForceSuspension)))

(fn GetDampingSuspension
  (return (Variables|SetupVehicle|GetDampingForce)))

(fn GetForwardInput
  (return (Math|Float|SelectFloat 0.0 (Variables|Private|GetForwardAxisVolue) (Math|Boolean|ORBoolean (Variables|Private|GetIsBreack) (Variables|Private|GetDeadCar) (> (Math|Float|Absolute(Float) (CallFunction|GetSpeed)) (Variables|Parametr|GetMaxSpeed))))))

(fn GetRightInput
  (return (Variables|Private|GetRightAxisVolue)))

(fn IsBreackInput
  (return (Variables|Private|GetIsBreack)))

(fn GetSpeed
  (bind _body (Variables|Default|GetBody))
  (bind _returnvalue (Class|PrimitiveComponent|GetPhysicsLinearVelocityatPoint _body (Transformation|GetWorldLocation _body) "None"))
  (return (* (.x (Math|Transform|InverseTransformDirection (Transformation|GetWorldTransform _body) _returnvalue)) 0.036)))

(fn SetRightVar
  (params (RightAxisVolue :type Float%20%28single-precision%29))
  (Variables|Private|SetRightAxisVolue RightAxisVolue))

(fn SetForwardVar
  (params (Value :type Float%20%28single-precision%29))
  (Variables|Private|SetForwardAxisVolue Value))

(fn IsDead
  (return (Variables|Private|GetDeadCar)))

(fn AddRotationWheels
  (for (_array_element _array_index) (Variables|Private|GetWheelsArr)
    (Transformation|AddLocalRotation _array_element (Math|Rotator|MakeRotator 0.0 (Variables|/Game/AllAssets/Blueprint/BPCarSimple/SimpleComponent.SimpleComponent_C|GetAngularVelocity (Utilities|Array|Get(acopy) (Variables|Private|GetComponentArr) _array_index)) 0.0) false false)))

(fn AddRotationWheel
  (for (_array_element _array_index) (Variables|Private|GetWheelsArr)
    (Transformation|AddLocalRotation _array_element (Math|Rotator|MakeRotator 0.0 (Variables|/Game/AllAssets/Blueprint/BPCarSimple/SimpleComponent.SimpleComponent_C|GetAngularVelocity (Utilities|Array|Get(acopy) (Variables|Private|GetComponentArr) _array_index)) 0.0) false false)
    (Transformation|SetWorldLocation _array_element (Math|Vector|MakeVector (.x (Transformation|GetWorldLocation _array_element)) (.y (Transformation|GetWorldLocation _array_element)) (.Z (Math|Vector|BreakVector (Variables|/Game/AllAssets/Blueprint/BPCarSimple/SimpleComponent.SimpleComponent_C|GetWheelLocation (Utilities|Array|Get(acopy) (Variables|Private|GetComponentArr) _array_index))))) true true)
    (Transformation|SetRelativeLocation _array_element (Math|Vector|MakeVector 0.0 0.0 (.z (Variables|/Script/Engine.SceneComponent|GetRelativeLocation _array_element))) true true)))