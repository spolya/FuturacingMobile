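; Simple raycast car physics component for AllCarPawn, providing suspension and throttle on the pawn's Box body.
; Each tick it line-traces down from every wheel socket and applies a mass-scaled spring plus damper force along the hit normal.
; Previous suspension distance and ground state are single variables shared by all wheels.
; Throttle adds forward acceleration when grounded, below max speed and not dead, with zero input while braking.
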(event EventBeginPlay
  (bind _asall_car_pawn (Utilities|Casting|CastToAllCarPawn (Components|GetOwner)))
  (bind _output_get (Variables|Default|SetParentCar _asall_car_pawn))
  (Variables|Default|SetBoxCarComponent (Variables|/Game/AllAssets/Blueprint/BPCarSimple/AllCarPawn.AllCarPawn_C|GetBox _output_get)))

(event EventTick
  (params (DeltaSeconds :type Float%20%28single-precision%29))
  (Variables|Default|SetDeltaTime DeltaSeconds)
  (CallFunction|UpdatePhysics))

(fn UpdatePhysics
  (for _array_element (Variables|WheelsSetup|GetWheelsSctruct)
    (Variables|Default|SetMeshWheel (.WheelMesh (Utilities|Struct|BreakWheelStructVehicle _array_element)))
    (Variables|Default|SetWheelSocketName (.SocketName (Utilities|Struct|BreakWheelStructVehicle _array_element)))
    (Variables|Default|SetRadiusWheel (.Radius (Utilities|Struct|BreakWheelStructVehicle _array_element)))
    (CallFunction|CreateLineTrace)
    (CallFunction|SuspensionForce)
    (Development|PrintString (Utilities|String|ToString(Float) (Variables|Default|GetZforce)) true true "(R=0.000000,G=0.660000,B=1.000000,A=1.000000)" 0.0)))

(fn StartedLoop)

(fn CreateLineTrace
  (bind _location (Utilities|GetLocationSocket))
  (bind (_outhit _returnvalue) (Collision|LineTraceForObjects _location (- _location (* (Math|Vector|GetUpVector (Variables|Default|GetBoxCarComponent)) (Variables|WheelsSetup|GetLengthSuspension))) (Utilities|Array|MakeArray "ObjectTypeQuery1") false (Utilities|Array|MakeArray (Variables|Default|GetParentCar)) "ForOneFrame"))
  (Variables|Default|SetBegraund_? _returnvalue)
  (if (Variables|Default|GetBegraund_?)
    (Variables|Default|SetDistanceSuspension (.Distance (Collision|BreakHitResult _outhit)))
    (Variables|Default|SetHitLocation (.Location (Collision|BreakHitResult _outhit)))
    (Variables|Default|SetHitNormal (.ImpactNormal (Collision|BreakHitResult _outhit)))
    (else
      (Variables|Default|SetDistanceSuspension (Variables|WheelsSetup|GetLengthSuspension)))))

(fn SuspensionForce
  ;[0.1754 1 0.9502 1 48] Suspresion Force
  ;;[1 1 1] Is Graund the Wheels
  (if (and (Variables|Default|GetBegraund_?) (Variables|/Game/AllAssets/Blueprint/BPCarSimple/AllCarPawn.AllCarPawn_C|GetUsePhysics (Variables|Default|GetParentCar)))
    (Variables|Default|SetZforce (+ (* (Math|Float|Lerp 1.0 0.0 (/ (Variables|Default|GetDistanceSuspension) (Variables|WheelsSetup|GetLengthSuspension))) (Variables|WheelsSetup|GetForceSuspension) (Physics|GetMass (Variables|/Game/AllAssets/Blueprint/BPCarSimple/AllCarPawn.AllCarPawn_C|GetBox (Variables|Default|GetParentCar))) 1e+02) (* (/ (- (Variables|Default|GetPreDistanceSuspension) (Variables|Default|GetDistanceSuspension)) (Variables|Default|GetDeltaTime)) (Variables|WheelsSetup|GetDampingForceSuspension))))
    (Class|PrimitiveComponent|AddForceatLocation (Variables|Default|GetBoxCarComponent) (* (Variables|Default|GetHitNormal) (Variables|Default|GetZforce)) (Transformation|GetSocketLocation (Variables|/Game/AllAssets/Blueprint/BPCarSimple/AllCarPawn.AllCarPawn_C|GetBody (Variables|Default|GetParentCar)) (Variables|Default|GetWheelSocketName)) "None")
    (else
      (Variables|Default|SetZforce 0.0)))
  (Variables|Default|SetWheelLocation (- (Utilities|GetLocationSocket) (* (Math|Vector|GetUpVector (Variables|Default|GetBoxCarComponent)) (Math|Float|Absolute(Float) (- (Variables|Default|GetDistanceSuspension) (Variables|Default|GetRadiusWheel))))))
  (Variables|Default|SetPreDistanceSuspension (Variables|Default|GetDistanceSuspension)))

(fn ThrotleInput
  (params (Axis :type Float%20%28single-precision%29))
  (bind _parentcar (Variables|Default|GetParentCar))
  (Variables|Default|SetMoveForward (* Axis (Math|Float|SelectFloat 0.0 1.0 (Variables|/Game/AllAssets/Blueprint/BPCarSimple/AllCarPawn.AllCarPawn_C|GetIsBreack (Variables|Default|GetParentCar)))))
  (if (Math|Boolean|ANDBoolean (< (Variables|/Game/AllAssets/Blueprint/BPCarSimple/AllCarPawn.AllCarPawn_C|GetSpeed _parentcar) (Variables|/Game/AllAssets/Blueprint/BPCarSimple/AllCarPawn.AllCarPawn_C|GetMaxSpeed _parentcar)) (Variables|Default|GetBegraund_?) (not (Variables|/Game/AllAssets/Blueprint/BPCarSimple/AllCarPawn.AllCarPawn_C|GetDeadCar _parentcar)))
    (Physics|AddForce (Variables|Default|GetBoxCarComponent) (* (Math|Vector|GetForwardVector (Variables|Default|GetBoxCarComponent)) (* (Variables|Default|GetMoveForward) (Variables|/Game/AllAssets/Blueprint/BPCarSimple/AllCarPawn.AllCarPawn_C|GetAcceleration (Variables|Default|GetParentCar)))) (Variables|Default|GetWheelSocketName) true)))