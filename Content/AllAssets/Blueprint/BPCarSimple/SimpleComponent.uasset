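; Per-wheel component for a simple raycast car on an AllCarPawn, applying that wheel's physics to the pawn's Body when UsePhysics is on.
; Each tick a downward trace drives spring-damper suspension impulses and computes wheel location and ground contact.
; While grounded, it adds optional engine force and steering torque, velocity-based friction and yaw damping.
; Dirt and steam emitters follow the tire contact point.
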(event EventBeginPlay
  (bind _asall_car_pawn (Utilities|Casting|CastToAllCarPawn (Components|GetOwner)))
  (bind _output_get (Variables|Default|SetCar _asall_car_pawn))
  (Variables|Default|SetBodyComponent (Variables|/Game/AllAssets/Blueprint/BPCarSimple/AllCarPawn.AllCarPawn_C|GetBody _output_get))
  (if (Variables|/Game/AllAssets/Blueprint/BPCarSimple/AllCarPawn.AllCarPawn_C|GetUsePhysics (Variables|Default|GetCar))
    (bind _returnvalue (Effects|SpawnEmitterAttached "/Game/AllAssets/Blueprint/BPCarSimple/WheelDurty.WheelDurty" self "None" "0, 0, 0" "0, 0,90.000000" "1.000000,1.000000,1.000000" "KeepRelativeOffset" true "AutoRelease"))
    (Variables|Default|SetParticle _returnvalue)
    (bind _returnvalue_2 (Effects|SpawnEmitterAttached "/Game/StarterContent/Particles/P_Steam_Lit.P_Steam_Lit" self "None" "0, 0, 0" "0, 0,90.000000" "1.000000,1.000000,1.000000" "KeepRelativeOffset" true "AutoRelease"))
    (Variables|Default|SetSkidEffect _returnvalue_2)))

(event EventTick
  (params (DeltaSeconds :type Float%20%28single-precision%29))
  (bind _particle (Variables|Default|GetParticle))
  (bind _skideffect (Variables|Default|GetSkidEffect))
  (if (Variables|/Game/AllAssets/Blueprint/BPCarSimple/AllCarPawn.AllCarPawn_C|GetUsePhysics (Variables|Default|GetCar))
    (Variables|Default|SetDeltaTime DeltaSeconds)
    (CallFunction|UpdatePhysics)
    (Utilities|IsValid _particle
      (:Is%20Valid
        (Transformation|SetWorldLocation _particle (+ (Variables|Default|GetTireConnect) "0, 0,5.000000") true true)
        (Components|Activation|SetActive _particle true false)
        (Utilities|IsValid _skideffect
          (:Is%20Valid
            (Transformation|SetWorldLocation _skideffect (+ (Variables|Default|GetTireConnect) "0, 0,5.000000") true true)
            (Components|Activation|SetActive _skideffect true false)))))))

(fn UpdatePhysics
  (CallFunction|SuspensionSetup)
  (CallFunction|EngineForce)
  (CallFunction|SteeringForce)
  (CallFunction|FrictionModel)
  (CallFunction|AntiRotationBody))

(fn SuspensionSetup
  (bind _returnvalue (Transformation|GetWorldLocation))
  (bind _car (Variables|Default|GetCar))
  (LocalVariables|SetLength (Default|GetLengthSuspension (Variables|Default|GetCar)))
  ;[0.334 0.337 1 1 48] Create LineTrice
  (bind (_outhit _returnvalue_2) (Collision|LineTraceForObjects _returnvalue (- _returnvalue (* (Math|Vector|GetUpVector) (LocalVariables|GetLength))) (Utilities|Array|MakeArray "ObjectTypeQuery1") false (Utilities|Array|MakeArray (Variables|Default|GetCar)) "None"))
  (bind _output_get (Variables|Default|Setgraunded _returnvalue_2))
  (if _output_get
    (Variables|Default|Setdistance (.Distance (Collision|BreakHitResult _outhit)))
    (Variables|Default|SetTireConnect (.Location (Collision|BreakHitResult _outhit)))
    (bind _output_get_2 (LocalVariables|SetNormalLocal (.ImpactNormal (Collision|BreakHitResult _outhit))))
    (Variables|Default|SetNormalLocation _output_get_2)
    ;[0.1754 1 0.9502 1 48] Suspresion Force
    (Variables|Default|SetZValueVelocity (+ (* (Math|Float|Lerp 1.0 0.0 (/ (Variables|Default|Getdistance) (LocalVariables|GetLength))) (Default|GetForceSuspension _car) (Variables|/Game/AllAssets/Blueprint/BPCarSimple/AllCarPawn.AllCarPawn_C|GetMassVehicle _car) 1e+02) (* (/ (- (Variables|Default|GetpreDistance) (Variables|Default|Getdistance)) (Variables|Default|GetDeltaTime)) (Default|GetDampingSuspension (Variables|Default|GetCar)))))
    (Physics|AddImpulseatLocation (Variables|Default|GetBodyComponent) (* (LocalVariables|GetNormalLocal) (+ (* (Math|Float|Lerp 1.0 0.0 (/ (Variables|Default|Getdistance) (LocalVariables|GetLength))) (Default|GetForceSuspension _car) (Variables|/Game/AllAssets/Blueprint/BPCarSimple/AllCarPawn.AllCarPawn_C|GetMassVehicle _car) 1e+02) (* (/ (- (Variables|Default|GetpreDistance) (Variables|Default|Getdistance)) (Variables|Default|GetDeltaTime)) (Default|GetDampingSuspension (Variables|Default|GetCar))))) (Transformation|GetWorldLocation) "None")
    (else
      (Variables|Default|Setdistance (LocalVariables|GetLength))))
  (Variables|Default|SetWheelLocation (- (Transformation|GetWorldLocation) (* (Math|Vector|GetUpVector) (- (Variables|Default|Getdistance) (Variables|WheelSetup|GetRadiusWheel)))))
  (Variables|Default|SetpreDistance (Variables|Default|Getdistance)))

(fn FrictionModel
  ;[0.5781 0 0] Is Graunded
  (if (Variables|Default|Getgraunded)
    ;[1 0.634 0] Convert World Velocity To Local Velocity
    (bind _returnvalue (Class|PrimitiveComponent|GetPhysicsLinearVelocityatPoint (Variables|Default|GetBodyComponent) (Transformation|GetWorldLocation) "None"))
    (LocalVariables|SetXVolue (.X (Math|Vector|BreakVector (Math|Transform|InverseTransformDirection (Transformation|GetWorldTransform) _returnvalue))))
    (bind _output_get (LocalVariables|SetYVolue (.Y (Math|Vector|BreakVector (Math|Transform|InverseTransformDirection (Transformation|GetWorldTransform) _returnvalue)))))
    ;[1 0.629 0] Angular Velocity Wheels
    (Variables|Default|SetYValueVelocity _output_get)
    (Variables|Default|SetAngularVelocity (Math|Trig|RadiansToDegrees (* (+ (/ (LocalVariables|GetXVolue) (/ (Variables|WheelSetup|GetRadiusWheel) 1e+02)) (Variables|Default|GetThrottleValue)) 0.0001 -1.0)))
    ;[0 0.368 1] Friction Force
    (Development|PrintString (Utilities|String|ToString(Float) (Math|Float|MapRangeClamped (Math|Float|Absolute(Float) (LocalVariables|GetYVolue)) 0.0 5e+02 2e+01 (Variables|/Game/AllAssets/Blueprint/BPCarSimple/AllCarPawn.AllCarPawn_C|GetFrictionScales (Variables|Default|GetCar)))) true true "(R=0.025073,G=1.000000,B=0.000000,A=1.000000)" 0.0)
    (Class|PrimitiveComponent|AddForceatLocation (Variables|Default|GetBodyComponent) (* (+ (* (Math|Vector|GetForwardVector) (Math|Float|SelectFloat 0.0 (* -1.0 (LocalVariables|GetXVolue) 0.1) (> (Math|Float|Absolute(Float) (Default|GetForwardInput (Variables|Default|GetCar))) 0.0))) (* (Math|Vector|GetRightVector) (* (LocalVariables|GetYVolue) -1.0 (Math|Float|MapRangeClamped (Math|Float|Absolute(Float) (LocalVariables|GetYVolue)) 0.0 5e+02 2e+01 (Variables|/Game/AllAssets/Blueprint/BPCarSimple/AllCarPawn.AllCarPawn_C|GetFrictionScales (Variables|Default|GetCar)))))) 1e+03) (Transformation|GetWorldLocation) "None")))

(fn SteeringForce
  (bind _car (Variables|Default|GetCar))
  (bind _car_2 (Variables|Default|GetCar))
  (bind _rightaxisvolue (Default|GetRightInput _car))
  (bind _returnvalue (Default|GetSpeed _car_2))
  (if (Variables|WheelSetup|GetuseSteer)
    (Variables|Default|SetAngleWheel (Math|Float|SelectFloat (Math|Float|Clamp(Float) (+ (* _rightaxisvolue 2.0) (Variables|Default|GetAngleWheel)) -45.0 45.0) (* (Variables|Default|GetAngleWheel) 0.75) (!= _rightaxisvolue 0.0)))
    (if (Variables|Default|Getgraunded)
      ;[1 1 1] ограничение по скорости
      (if (> (Math|Float|Absolute(Float) (Default|GetSpeed (Variables|Default|GetCar))) 5.0)
        (Class|PrimitiveComponent|AddTorqueinRadians (Variables|Default|GetBodyComponent) (* (Math|Vector|GetUpVector (Variables|Default|GetBodyComponent)) (* (Default|GetRightInput (Variables|Default|GetCar)) (Variables|/Game/AllAssets/Blueprint/BPCarSimple/AllCarPawn.AllCarPawn_C|GetSteering (Variables|Default|GetCar)) (Math|Float|MapRangeUnclamped (Math|Float|Absolute(Float) _returnvalue) 0.0 8e+01 1.0 0.5) (Math|Float|MapRangeUnclamped _returnvalue -1e+01 1e+01 -1.0 1.0) 1.0)) "None" true)))))

(fn AntiRotationBody
  (bind _bodycomponent (Variables|Default|GetBodyComponent))
  (bind _bodycomponent_2 (Variables|Default|GetBodyComponent))
  (if (Variables|Default|Getgraunded)
    (Class|PrimitiveComponent|AddTorqueinRadians _bodycomponent_2 (* (Math|Vector|GetUpVector _bodycomponent_2) (* (Math|Float|MapRangeUnclamped (Variables|/Game/AllAssets/Blueprint/BPCarSimple/AllCarPawn.AllCarPawn_C|GetFrictionScales (Variables|Default|GetCar)) 0.0 1e+01 0.0 1.0) -1.0 (.Z (Math|Vector|BreakVector (Math|Transform|InverseTransformDirection (Transformation|GetWorldTransform _bodycomponent) (Class|PrimitiveComponent|GetPhysicsAngularVelocityinRadians _bodycomponent "None")))))) "None" true)))

(fn EngineForce
  (bind _bodycomponent (Variables|Default|GetBodyComponent))
  (bind _car (Variables|Default|GetCar))
  (bind _car_2 (Variables|Default|GetCar))
  (bind _forwardaxisvolue (Default|GetForwardInput _car_2))
  (bind _returnvalue (Default|GetSpeed _car_2))
  (if (and (Variables|Default|Getgraunded) (Variables|Default|GetUseForce))
    (Variables|Default|SetThrottleValue (* (Math|Float|SelectFloat _forwardaxisvolue (* _forwardaxisvolue 2.0) (or (and (> _forwardaxisvolue 0.0) (> _returnvalue 0.0)) (and (< _forwardaxisvolue 0.0) (< _returnvalue 0.0)))) (Variables|/Game/AllAssets/Blueprint/BPCarSimple/AllCarPawn.AllCarPawn_C|GetAcceleration (Variables|Default|GetCar)) 1e+04 (- 1.0 (/ (Math|Float|Absolute(Float) (Default|GetSpeed _car)) (Variables|/Game/AllAssets/Blueprint/BPCarSimple/AllCarPawn.AllCarPawn_C|GetMaxSpeed _car)))))
    (Class|PrimitiveComponent|AddForceatLocation _bodycomponent (* (Math|Vector|GetForwardVector (Variables|Default|GetBodyComponent)) (Variables|Default|GetThrottleValue)) (Transformation|GetWorldLocation _bodycomponent) "None")))

(fn TruePhysics
  (Utilities|Time|SetTimerbyFunctionName 0 "UpdatePhysics" (Variables|Default|GetDeltaTime) true))