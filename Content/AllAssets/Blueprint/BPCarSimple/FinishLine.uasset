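; Race manager actor at the finish line that counts laps, ends the race and runs the player HUD with a live leaderboard.
; Box overlap advances a car's lap once it has enough checkpoints and clears checkpoint ignore lists; on the last lap the player gets the finish screen, AI cars get flagged finished.
; Tick scores cars by lap plus closest track-spline key, then ranks them by repeatedly taking and zeroing the maximum score.
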(event OnComponentBeginOverlap(Box)
  (params (OverlappedComponent :type Primitive%20Component%20Object%20Reference) (OtherActor :type Actor%20Object%20Reference) (OtherComp :type Primitive%20Component%20Object%20Reference) (OtherBodyIndex :type Integer) (bFromSweep :type Boolean) (SweepResult :type Hit%20Result%20Structure%20%28by%20ref%29))
  (bind _asall_car_pawn (Utilities|Casting|CastToAllCarPawn OtherActor))
  (if (>= (Variables|/Game/AllAssets/Blueprint/BPCarSimple/AllCarPawn.AllCarPawn_C|GetNumberCheckPoint _asall_car_pawn) (Variables|Default|GetMaxCheckPoint))
    (if (>= (Variables|/Game/AllAssets/Blueprint/BPCarSimple/AllCarPawn.AllCarPawn_C|GetNumberCircle _asall_car_pawn) (Variables|Default|GetMaxCircle))
      (if (Pawn|IsPlayerControlled _asall_car_pawn)
        (Input|DisableInput _asall_car_pawn (Game|GetPlayerController 0))
        (Default|SetForwardVar _asall_car_pawn 0.0)
        (Default|SetRightVar _asall_car_pawn 0.0)
        (Viewport|RemoveAllWidgets)
        (bind _returnvalue (UserInterface|CreateWidget "/Game/AllAssets/Blueprint/BPCarSimple/FinishUMG.FinishUMG_C"))
        (UserInterface|Viewport|AddtoViewport _returnvalue 0)
        (else
          (Variables|/Game/AllAssets/Blueprint/BPCarSimple/AllCarPawn.AllCarPawn_C|SetFinished _asall_car_pawn true)))
      (else
        (Variables|/Game/AllAssets/Blueprint/BPCarSimple/AllCarPawn.AllCarPawn_C|SetNumberCircle _asall_car_pawn (+ (Variables|/Game/AllAssets/Blueprint/BPCarSimple/AllCarPawn.AllCarPawn_C|GetNumberCircle _asall_car_pawn) 1))
        (for _array_element (Variables|Default|GetCheckPoints)
          (Utilities|Array|Clear (Variables|/Game/AllAssets/Blueprint/BPCarSimple/CheckPoint.CheckPoint_C|GetignoreVehicle _array_element)))
        (CallFunction|UpdateDataCirclePlayer)))))

(event EventBeginPlay
  (bind _outactors (Actor|GetAllActorsOfClass "/Game/AllAssets/Blueprint/BPCarSimple/CheckPoint.CheckPoint_C"))
  (Variables|Default|SetCheckPoints _outactors)
  (Variables|Default|SetMaxCheckPoint (Utilities|Array|Length _outactors))
  (bind _outactors_2 (Actor|GetAllActorsOfClass "/Game/AllAssets/Blueprint/BPCarSimple/SplineTrack.SplineTrack_C"))
  (Variables|Default|SetSplinePath (Utilities|Array|Get(acopy) _outactors_2))
  (bind _returnvalue (UserInterface|CreateWidget "/Game/AllAssets/Blueprint/BPCarSimple/HUDplayer/PlayerHUDwidget.PlayerHUDwidget_C" (Game|GetPlayerController 0)))
  (Variables|Default|SetHUD _returnvalue)
  (UserInterface|Viewport|AddtoViewport _returnvalue 0)
  (CallFunction|UpdateDataCirclePlayer)
  (bind _outactors_3 (Actor|GetAllActorsOfClass "/Game/AllAssets/Blueprint/BPCarSimple/AllCarPawn.AllCarPawn_C"))
  (bind _output_get (Variables|Default|SetAllCar _outactors_3))
  (for _array_element _output_get
    (Utilities|Array|Add (Variables|Default|GetTotalTime) 0.0)
    (bind _returnvalue_2 (UserInterface|CreateWidget "/Game/AllAssets/Blueprint/BPCarSimple/HUDplayer/TextLiderList.TextLiderList_C" (Game|GetPlayerController 0)))
    (Class|VerticalBox|AddChildtoVerticalBox (Variables|/Game/AllAssets/Blueprint/BPCarSimple/HUDplayer/PlayerHUDwidget.PlayerHUDwidget_C|GetLiderList (Variables|Default|GetHUD)) _returnvalue_2)))

(event EventTick
  (params (DeltaSeconds :type Float%20%28single-precision%29))
  (bind _splinepath (Variables|Default|GetSplinePath))
  (bind _totaltime (Variables|Default|GetTotalTime))
  (bind _allcar (Variables|Default|GetAllCar))
  (bind _indexofmaxvalue (Math|Float|MaxOfFloatArray _totaltime))
  (bind _spline (Variables|/Game/AllAssets/Blueprint/BPCarSimple/SplineTrack.SplineTrack_C|GetSpline _splinepath))
  (bind _output (Utilities|Array|Get(acopy) _allcar _indexofmaxvalue))
  (bind _returnvalue (Pawn|IsPlayerControlled _output))
  (Utilities|IsValid (Variables|Default|GetSplinePath)
    (:Is%20Valid
      (for (_array_element _array_index) (Variables|Default|GetAllCar)
        (bind _output_get (Variables|Default|SetSelectCar _array_element))
        (Utilities|IsValid _output_get
          (:Is%20Valid
            (Utilities|Array|SetArrayElem (Variables|Default|GetTotalTime) _array_index (+ (/ (Class|SplineComponent|FindInputKeyClosesttoWorldLocation _spline (Spline|FindLocationClosesttoWorldLocation (Variables|/Game/AllAssets/Blueprint/BPCarSimple/SplineTrack.SplineTrack_C|GetSpline (Variables|Default|GetSplinePath)) (Transformation|GetWorldLocation (Variables|/Game/AllAssets/Blueprint/BPCarSimple/AllCarPawn.AllCarPawn_C|GetBody _array_element)) "World")) (Math|Conversions|ToFloat(Integer) (Spline|GetNumberOfSplinePoints _spline))) (Math|Conversions|ToFloat(Integer) (Variables|/Game/AllAssets/Blueprint/BPCarSimple/AllCarPawn.AllCarPawn_C|GetNumberCircle (Variables|Default|GetSelectCar))))))))
      (for (_ _array_index_2) (Variables|Default|GetAllCar)
        (Utilities|IsValid _output
          (:Is%20Valid
            (if (and (not (Variables|/Game/AllAssets/Blueprint/BPCarSimple/AllCarPawn.AllCarPawn_C|GetFinished _output)) _returnvalue)
              (Variables|Default|SetPlayerPosition (+ _array_index_2 1)))
            (bind _astext_lider_list (Utilities|Casting|CastToTextLiderList (Class|PanelWidget|GetChildat (Variables|/Game/AllAssets/Blueprint/BPCarSimple/HUDplayer/PlayerHUDwidget.PlayerHUDwidget_C|GetLiderList (Variables|Default|GetHUD)) _array_index_2)))
            (Rendering|Components|TextRender|SetText (Variables|/Game/AllAssets/Blueprint/BPCarSimple/HUDplayer/TextLiderList.TextLiderList_C|Gettext _astext_lider_list) (Utilities|Text|ToText(String) (Utilities|String|Append (Utilities|String|ToString(Integer) (+ _array_index_2 1)) " . " (Utilities|String|SelectString "You" (Utilities|String|ToString(Name) (Variables|/Game/AllAssets/Blueprint/BPCarSimple/AllCarPawn.AllCarPawn_C|GetNameCar _output)) _returnvalue))))
            (Utilities|Array|SetArrayElem (Variables|Default|GetTotalTime) _indexofmaxvalue 0.0)))))))

(fn ConstructionScript)

(fn UpdateDataCirclePlayer
  (bind _asall_car_pawn (Utilities|Casting|CastToAllCarPawn (Game|Player|GetPlayerPawn 0)))
  (Rendering|Components|TextRender|SetText (Variables|/Game/AllAssets/Blueprint/BPCarSimple/HUDplayer/PlayerHUDwidget.PlayerHUDwidget_C|GetCircleData (Variables|Default|GetHUD)) (Utilities|Text|ToText(String) (Utilities|String|Append "Круг: " (Utilities|String|ToString(Integer) (Variables|/Game/AllAssets/Blueprint/BPCarSimple/AllCarPawn.AllCarPawn_C|GetNumberCircle _asall_car_pawn)) "/" (Utilities|String|ToString(Integer) (Variables|Default|GetMaxCircle))))))