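; Spline-based car track actor that lays collidable spline meshes along its path and provides path points for AI cars.
; FuncUpdate builds the segments in construction when UpdateSpline is set and again on BeginPlay, which also caches all car pawns.
; PlayAISplinePath loops a fast timer on SetSteerVehicle, storing a spline point near LocalCar, offset along a rotated track right vector.
; GetLocationCar returns any vehicle's closest spline point.
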(event EventBeginPlay
  (Variables|Default|SetUpdateSpline true)
  (CallFunction|FuncUpdate)
  (bind _outactors (Actor|GetAllActorsOfClass "/Game/AllAssets/Blueprint/BPCarSimple/AllCarPawn.AllCarPawn_C"))
  (Variables|Default|SetAllCarArr _outactors))

(fn ConstructionScript
  (CallFunction|FuncUpdate))

(fn FuncUpdate
  (bind _addmesh (Variables|Default|GetAddMesh))
  (bind _tangentscale (Variables|Default|GetTangentScale))
  (bind _spline (Variables|Default|GetSpline))
  (if (Variables|Default|GetUpdateSpline)
    (for _index (range 0 (Math|Float|Truncate (/ (Spline|GetSplineLength (Variables|Default|GetSpline)) (Variables|Default|GetAddMesh))))
      (bind _returnvalue (AddComponent|AddSplineMeshComponent true))
      (Components|StaticMesh|SetStaticMesh _returnvalue (Variables|Default|GetMesh))
      (Collision|SetCollisionEnabled _returnvalue "QueryAndPhysics")
      (Collision|SetCollisionObjectType _returnvalue "ECC_WorldStatic")
      (SplineMesh|SetStartandEnd _returnvalue (Spline|GetLocationatDistanceAlongSpline _spline (* _index _addmesh) "World") (* (Spline|GetDirectionatDistanceAlongSpline _spline (* _index _addmesh) "World") _tangentscale) (Spline|GetLocationatDistanceAlongSpline _spline (+ (* _index _addmesh) _addmesh) "World") (* (Spline|GetDirectionatDistanceAlongSpline _spline (+ (* _index _addmesh) _addmesh) "World") _tangentscale) true :!class /Script/Engine.SplineMeshComponent)
      (Spline|SetClosedLoop (Variables|Default|GetSpline) (Variables|Default|GetLoopSpline) true)
      (Class|PrimitiveComponent|SetCullDistance _returnvalue (Variables|Default|GetCullDistance))
      (Variables|Default|SetUpdateSpline false))))

(fn SetSteerVehicle
  (bind _localcar (Variables|Default|GetLocalCar))
  (bind _spline (Variables|Default|GetSpline))
  (bind _box (Variables|/Game/AllAssets/Blueprint/BPCarSimple/AllCarPawn.AllCarPawn_C|GetBox _localcar))
  (bind _returnvalue (Transformation|GetWorldLocation _box))
  (bind _returnvalue_2 (Class|SplineComponent|FindRightVectorClosesttoWorldLocation _spline _returnvalue "Local"))
  (bind _returnvalue_3 (Math|Rotator|MakeRotationfromAxes _returnvalue_2 "0, 0, 0" "0, 0, 0"))
  (bind (_roll _pitch _yaw) (Math|Rotator|BreakRotator _returnvalue_3))
  (Utilities|IsValid (Variables|Default|GetLocalCar)
    (:Is%20Valid
      (Variables|Default|SetLocalCorrect (Spline|FindLocationClosesttoWorldLocation (Variables|Default|GetSpline) (- (Transformation|GetWorldLocation (Variables|/Game/AllAssets/Blueprint/BPCarSimple/AllCarPawn.AllCarPawn_C|GetBox (Variables|Default|GetLocalCar))) (* (Math|Vector|GetForwardVector (Math|Rotator|MakeRotator _roll _pitch (+ _yaw (Variables|Default|GetAddRotateForward)))) 5500)) "World")))))

(fn PlayAISplinePath
  (Utilities|Time|SetTimerbyFunctionName 0 "SetSteerVehicle" 0.01 true))

(fn GetLocationCar
  (params (Vehicle :type All%20Car%20Pawn%20Object%20Reference))
  (return (Spline|FindLocationClosesttoWorldLocation (Variables|Default|GetSpline) (Transformation|GetWorldLocation (Variables|/Game/AllAssets/Blueprint/BPCarSimple/AllCarPawn.AllCarPawn_C|GetBox Vehicle)) "World")))