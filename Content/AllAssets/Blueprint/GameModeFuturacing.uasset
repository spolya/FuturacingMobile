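; Game mode for a racing game that keeps persistent player progress, shop car and weapon data, currencies and settings.
; BeginPlay loads SaveSlot1 from slot "1" into its variables, or creates and saves one from current values when none loads.
; It then applies music and effect volumes through sound mix overrides, and also runs the Stat FPS console command.
; EndPlay copies the variables back into the save object and writes the slot.
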(event EventBeginPlay
  (bind _returnvalue (Game|GetPlayerController 0))
  (Development|ExecuteConsoleCommand _returnvalue "Stat FPS" _returnvalue)
  (bind _returnvalue_2 (SaveGame|LoadGamefromSlot "1"))
  (bind _assave_slot_1 (Utilities|Casting|CastToSaveSlot1 _returnvalue_2)
    (:then
      (Variables|Default|SetSave _assave_slot_1)
      (CallFunction|LoadSave))
    (:CastFailed
      (bind _returnvalue_3 (SaveGame|CreateSaveGameObject "/Game/AllAssets/Blueprint/SaveSlot1.SaveSlot1_C"))
      (CallFunction|SaveGame _returnvalue_3)))
  (Audio|SetSoundMixClassOverride "/Game/AllAssets/SaundDiz/GameSoundMix.GameSoundMix" "/Game/AllAssets/SaundDiz/SoundMusik.SoundMusik" (Variables|Default|GetMusicScale) 1.0 1.0 true)
  (Audio|SetSoundMixClassOverride "/Game/AllAssets/SaundDiz/GameSoundMix.GameSoundMix" "/Game/AllAssets/SaundDiz/SoundEffect.SoundEffect" (Variables|Default|GetEffectScale) 1.0 1.0 true))

(event EventEndPlay
  (params (EndPlayReason :type EEndPlayReason%20Enum :default "Destroyed"))
  (CallFunction|SaveGame (Variables|Default|GetSave)))

(fn ConstructionScript)

(fn SaveGame
  (params (Save :type Save%20Slot%201%20Object%20Reference))
  (bind _output_get (Variables|Default|SetSave Save))
  (Variables|/Game/AllAssets/Blueprint/SaveSlot1.SaveSlot1_C|SetArrCar _output_get (Variables|Default|GetMagazineCar))
  (Variables|/Game/AllAssets/Blueprint/SaveSlot1.SaveSlot1_C|SetArrGun (Variables|Default|GetSave) (Variables|Default|GetMagazineWeapon))
  (Variables|/Game/AllAssets/Blueprint/SaveSlot1.SaveSlot1_C|SetValueMusic (Variables|Default|GetSave) (Variables|Default|GetMusicScale))
  (Variables|/Game/AllAssets/Blueprint/SaveSlot1.SaveSlot1_C|SetValueEffect (Variables|Default|GetSave) (Variables|Default|GetEffectScale))
  (Variables|/Game/AllAssets/Blueprint/SaveSlot1.SaveSlot1_C|SetFCoins (Variables|Default|GetSave) (Variables|Player|GetPlayerFcoins))
  (Variables|/Game/AllAssets/Blueprint/SaveSlot1.SaveSlot1_C|SetSFCoins (Variables|Default|GetSave) (Variables|Player|GetPlayerSFcoins))
  (Variables|/Game/AllAssets/Blueprint/SaveSlot1.SaveSlot1_C|SetAutoBreack (Variables|Default|GetSave) (Variables|Player|GetPlayerAutobreack))
  (Variables|/Game/AllAssets/Blueprint/SaveSlot1.SaveSlot1_C|SetControllerType (Variables|Default|GetSave) (Variables|Player|GetPlayerControlledType))
  (Variables|/Game/AllAssets/Blueprint/SaveSlot1.SaveSlot1_C|SetIndexCar (Variables|Default|GetSave) (Variables|Player|GetPlayerCarIndex))
  (Variables|/Game/AllAssets/Blueprint/SaveSlot1.SaveSlot1_C|SetIndexGun (Variables|Default|GetSave) (Variables|Player|GetPlayerWeaponIndex))
  (Variables|/Game/AllAssets/Blueprint/SaveSlot1.SaveSlot1_C|SetPlayerXP (Variables|Default|GetSave) (Variables|Player|GetPlayerXP))
  (Variables|/Game/AllAssets/Blueprint/SaveSlot1.SaveSlot1_C|SetRedMicro (Variables|Default|GetSave) (Variables|Player|GetPlayerRedMicro))
  (Variables|/Game/AllAssets/Blueprint/SaveSlot1.SaveSlot1_C|SetGreenMicro (Variables|Default|GetSave) (Variables|Player|GetPlayerGreenMicro))
  (Variables|/Game/AllAssets/Blueprint/SaveSlot1.SaveSlot1_C|SetPeopleMicro (Variables|Default|GetSave) (Variables|Player|GetPlayerPeopleMicro))
  (Variables|/Game/AllAssets/Blueprint/SaveSlot1.SaveSlot1_C|SetNumberRace (Variables|Default|GetSave) (Variables|Player|GetPlayerNumberRace))
  (SaveGame|SaveGametoSlot (Variables|Default|GetSave) "1"))

(fn LoadSave
  (Variables|Default|SetMagazineCar (Variables|/Game/AllAssets/Blueprint/SaveSlot1.SaveSlot1_C|GetArrCar (Variables|Default|GetSave)))
  (Variables|Default|SetMagazineWeapon (Variables|/Game/AllAssets/Blueprint/SaveSlot1.SaveSlot1_C|GetArrGun (Variables|Default|GetSave)))
  (Variables|Default|SetMusicScale (Variables|/Game/AllAssets/Blueprint/SaveSlot1.SaveSlot1_C|GetValueMusic (Variables|Default|GetSave)))
  (Variables|Default|SetEffectScale (Variables|/Game/AllAssets/Blueprint/SaveSlot1.SaveSlot1_C|GetValueEffect (Variables|Default|GetSave)))
  (Variables|Player|SetPlayerFcoins (Variables|/Game/AllAssets/Blueprint/SaveSlot1.SaveSlot1_C|GetFCoins (Variables|Default|GetSave)))
  (Variables|Player|SetPlayerSFcoins (Variables|/Game/AllAssets/Blueprint/SaveSlot1.SaveSlot1_C|GetSFCoins (Variables|Default|GetSave)))
  (Variables|Player|SetPlayerCarIndex (Variables|/Game/AllAssets/Blueprint/SaveSlot1.SaveSlot1_C|GetIndexCar (Variables|Default|GetSave)))
  (Variables|Player|SetPlayerWeaponIndex (Variables|/Game/AllAssets/Blueprint/SaveSlot1.SaveSlot1_C|GetIndexGun (Variables|Default|GetSave)))
  (Variables|Player|SetPlayerControlledType (Variables|/Game/AllAssets/Blueprint/SaveSlot1.SaveSlot1_C|GetControllerType (Variables|Default|GetSave)))
  (Variables|Player|SetPlayerAutobreack (Variables|/Game/AllAssets/Blueprint/SaveSlot1.SaveSlot1_C|GetAutoBreack (Variables|Default|GetSave)))
  (Variables|Player|SetPlayerXP (Variables|/Game/AllAssets/Blueprint/SaveSlot1.SaveSlot1_C|GetPlayerXP (Variables|Default|GetSave)))
  (Variables|Player|SetPlayerRedMicro (Variables|/Game/AllAssets/Blueprint/SaveSlot1.SaveSlot1_C|GetRedMicro (Variables|Default|GetSave)))
  (Variables|Player|SetPlayerGreenMicro (Variables|/Game/AllAssets/Blueprint/SaveSlot1.SaveSlot1_C|GetGreenMicro (Variables|Default|GetSave)))
  (Variables|Player|SetPlayerPeopleMicro (Variables|/Game/AllAssets/Blueprint/SaveSlot1.SaveSlot1_C|GetPeopleMicro (Variables|Default|GetSave)))
  (Variables|Player|SetPlayerNumberRace (Variables|/Game/AllAssets/Blueprint/SaveSlot1.SaveSlot1_C|GetNumberRace (Variables|Default|GetSave))))