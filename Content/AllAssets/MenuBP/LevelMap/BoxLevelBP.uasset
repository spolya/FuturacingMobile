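; BoxLevelBP is a touchable level-select box that opens its assigned level when unlocked.
; The construction script labels it with LevelNumber and colors the text red if ToOpen is set, black otherwise.
; Touching the cube either runs Loading, which shows a loading screen, locks input to UI and opens LevelOpen after a short delay, or shows a Warning widget carrying the previous level's number.
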(event OnInputTouchBegin(Cube)
  (params (FingerIndex :type ETouchIndex%20Enum :default "Touch1") (TouchedComponent :type Primitive%20Component%20Object%20Reference))
  (CallFunction|OpentoLevel))

(event Custom|Loading
  (bind _returnvalue (Game|GetPlayerController 0))
  (bind _returnvalue_2 (UserInterface|CreateWidget "/Game/AllAssets/MenuBP/LoadingScreen.LoadingScreen_C"))
  (UserInterface|Viewport|AddtoViewport _returnvalue_2 0)
  (Variables|/Script/Engine.PlayerController|SetbShowMouseCursor _returnvalue false)
  (Input|SetInputModeUIOnly _returnvalue _returnvalue_2 "LockAlways")
  (Utilities|FlowControl|Delay 0.2)
  (Game|OpenLevel(byName) (Variables|Default|GetLevelOpen)))

(fn ConstructionScript
  (bind _textrender (Variables|Default|GetTextRender))
  (Rendering|Components|TextRender|SetText _textrender (Utilities|Text|ToText(String) (Utilities|String|Append "Level: " (Utilities|String|ToString(Integer) (Variables|Default|GetLevelNumber)))))
  (Rendering|Components|TextRender|SetTextRenderColor _textrender (select (Variables|Default|GetToOpen) (Math|Color|MakeColor 0 0 255 255) (Math|Color|MakeColor 0 0 0 255))))

(fn OpentoLevel
  (if (Variables|Default|GetToOpen)
    (CallFunction|Loading)
    (else
      (bind _returnvalue (UserInterface|CreateWidget "/Game/AllAssets/MenuBP/LevelMap/Warning.Warning_C"))
      (Variables|/Game/AllAssets/MenuBP/LevelMap/Warning.Warning_C|SetNumberLevel _returnvalue (- (Variables|Default|GetLevelNumber) 1))
      (UserInterface|Viewport|AddtoViewport _returnvalue 0))))