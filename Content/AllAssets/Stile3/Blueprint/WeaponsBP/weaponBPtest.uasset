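; Auto-firing turret weapon that reads its parent PawnXY car and stops attacking and tracking once that car is dead.
; Each tick it scans all PawnXY for a living target in range, favoring closer ones, and interpolates the mesh yaw toward it.
; A looping timer spends ammo on hitscan traces that apply damage and spawn a beam trail.
; Touching its box triggers the CameraTarget pawn's camera animation; a debug line shows the player's target.
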(event OnInputTouchBegin(Box)
  (params (FingerIndex :type ETouchIndex%20Enum :default "Touch1") (TouchedComponent :type Primitive%20Component%20Object%20Reference))
  (Development|PrintString "Hello" true true "(R=0.437500,G=0.000000,B=0.150380,A=1.000000)")
  (bind _ascamera_target (Utilities|Casting|CastToCameraTarget (Game|Player|GetPlayerPawn 0)))
  (Default|AnimationCamera _ascamera_target))

(event EventTick
  (params (DeltaSeconds :type Float%20%28single-precision%29))
  (Variables|Private|SetDeltaTime DeltaSeconds)
  (if (Variables|/Game/BPCarSimple/PawnXY.PawnXY_C|GetDeadCar (Variables|Private|GetParentActor))
    (Utilities|Time|ClearTimerbyFunctionName 0 "AttackToTarget")
    (else
      (CallFunction|GetActorTarget)
      (CallFunction|RotateWeapontoTarget)
      (CallFunction|DebugOnly))))

(event EventBeginPlay
  (CallFunction|StartINI)
  (Utilities|Time|SetTimerbyFunctionName 0 "AttackToTarget" (- 1.0 (Variables|Default|GetTimeAttack)) true))

(fn ConstructionScript)

(fn GetActorTarget
  (bind _outactors (Actor|GetAllActorsOfClass "/Game/BPCarSimple/PawnXY.PawnXY_C"))
  (for _array_element _outactors
    (Variables|Private|SetLastTargetActor _array_element)
    (Utilities|IsValid (Variables|Private|GetTargetActor)
      (:Is%20Valid
        (if (Math|Boolean|ANDBoolean (< (Transformation|GetDistanceTo (Variables|Private|GetTargetActor) self) (Variables|Default|GetLengthAttack)) (not (Variables|/Game/BPCarSimple/PawnXY.PawnXY_C|GetDeadCar (Variables|Private|GetTargetActor))) (!= (Variables|Private|GetTargetActor) (Variables|Private|GetParentActor)))
          (if (Math|Boolean|ANDBoolean (< (Transformation|GetDistanceTo (Variables|Private|GetLastTargetActor) self) (Variables|Default|GetLengthAttack)) (> (Transformation|GetDistanceTo (Variables|Private|GetLastTargetActor) self) 1.5e+02) (not (Variables|/Game/BPCarSimple/PawnXY.PawnXY_C|GetDeadCar (Variables|Private|GetLastTargetActor))) (!= (Variables|Private|GetLastTargetActor) (Variables|Private|GetParentActor)))
            (if (> (Transformation|GetDistanceTo (Variables|Private|GetTargetActor) self) (Transformation|GetDistanceTo (Variables|Private|GetLastTargetActor) self))
              (Variables|Private|SetTargetActor (Variables|Private|GetLastTargetActor) :!label _label)))
          (else
            (if (Math|Boolean|ANDBoolean (< (Transformation|GetDistanceTo (Variables|Private|GetLastTargetActor) self) (Variables|Default|GetLengthAttack)) (> (Transformation|GetDistanceTo (Variables|Private|GetLastTargetActor) self) 1.5e+02) (not (Variables|/Game/BPCarSimple/PawnXY.PawnXY_C|GetDeadCar (Variables|Private|GetLastTargetActor))) (!= (Variables|Private|GetLastTargetActor) (Variables|Private|GetParentActor))) :!label _label_2
              (goto _label)
              (else
                (Variables|Private|SetTargetActor 0))))))
      (:Is%20Not%20Valid
        (goto _label_2)))))

(fn DebugOnly
  (Utilities|IsValid (Variables|Private|GetTargetActor)
    (:Is%20Valid
      (if (== (Variables|Private|GetParentActor) (Game|Player|GetPlayerPawn 0))
        (Rendering|Debug|DrawDebugLine :LineStart (Transformation|GetActorLocation) :LineEnd (Transformation|GetActorLocation (Variables|Private|GetTargetActor)) :Thickness 5.0)))))

(fn RotateWeapontoTarget
  (Utilities|IsValid (Variables|Private|GetTargetActor)
    (:Is%20Valid
      ;[0.2812 0.2812 0.2812 1 36] Поворот башни к цели
      (Transformation|SetRelativeRotation (Variables|Default|GetStaticMesh) (Math|Rotator|MakeRotator 0.0 -5.0 (.Yaw (Math|Rotator|BreakRotator (Math|Interpolation|RInterpTo (Variables|/Script/Engine.SceneComponent|GetRelativeRotation (Variables|Default|GetStaticMesh)) (Math|Rotator|Delta(Rotator) (Math|Rotator|FindLookatRotation (Transformation|GetActorLocation) (Transformation|GetActorLocation (Variables|Private|GetTargetActor))) (Transformation|GetActorRotation)) (Variables|Private|GetDeltaTime) (* (Variables|Default|GetTimeRotate) 1e+01))))) true false))
    (:Is%20Not%20Valid
      ;[1 1 1 1 36] Поворот башни в исходное положение
      (Transformation|SetRelativeRotation (Variables|Default|GetStaticMesh) (Math|Interpolation|RInterpTo (Variables|/Script/Engine.SceneComponent|GetRelativeRotation (Variables|Default|GetStaticMesh)) "0.000000, 0, 0" (Variables|Private|GetDeltaTime) (* (Variables|Default|GetTimeRotate) 1e+01)) true false))))

(fn StartINI
  (bind _aspawn_xy (Utilities|Casting|CastToPawnXY (Actor|GetParentActor self)))
  (Variables|Private|SetParentActor _aspawn_xy))

(fn AttacktoTarget
  (bind _sphere (Variables|Default|GetSphere))
  (bind _returnvalue (Transformation|GetWorldLocation _sphere))
  ;[0.25 0.25 0.25 1 36] Наличие цели амуниции и ее расход
  (if (and (Utilities|IsValid (Variables|Private|GetTargetActor)) (> (Variables|Default|GetAmmunication) 0))
    (Variables|Default|SetAmmunication (- (Variables|Default|GetAmmunication) 1))
    ;[0.3073 0.3073 0.3073 1 36] Отрисовка луча
    (bind _outhit (Collision|LineTraceByChannel _returnvalue (+ _returnvalue (* (Math|Vector|GetForwardVector _sphere) 1500)) "TraceTypeQuery1" false (Utilities|Array|MakeArray (Variables|Private|GetParentActor)) "ForOneFrame"))
    (Variables|Default|SetHit (.bBlockingHit (Collision|BreakHitResult _outhit)))
    (Variables|Default|SetPointHit (.ImpactPoint (Collision|BreakHitResult _outhit)))
    (Variables|Default|SetActorHit (.HitActor (Collision|BreakHitResult _outhit)))
    (Variables|Default|SetStartPoint (.TraceStart (Collision|BreakHitResult _outhit)))
    ;[0.4167 0.4167 0.4167 1 36] Нанесение урона
    (Variables|Default|SetEndPoint (.TraceEnd (Collision|BreakHitResult _outhit)))
    (Game|Damage|ApplyDamage (Variables|Default|GetActorHit) (Variables|Default|GetDamage) 0 0)
    ;[0.3698 0.3698 0.3698 1 36] Создание Частиц
    (bind _returnvalue_2 (Effects|SpawnEmitteratLocation "/Game/Effects/ParticleSystems/Weapons/AssaultRifle/Muzzle/P_AssaultRifle_Trail.P_AssaultRifle_Trail" (Variables|Default|GetStartPoint) (Math|Conversions|RotationFromXVector (Variables|Default|GetStartPoint))))
    (Effects|Components|ParticleSystem|SetVectorParameter _returnvalue_2 "ShockBeamEnd" (Math|Vector|SelectVector (Variables|Default|GetPointHit) (Variables|Default|GetEndPoint) (Variables|Default|GetHit)))))